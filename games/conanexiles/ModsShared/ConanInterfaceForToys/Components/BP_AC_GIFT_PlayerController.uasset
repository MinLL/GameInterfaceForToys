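; Player controller component of the GIFT toy interface mod for Conan Exiles that turns toy events and custom data into client log lines.
; Interface calls validate the event row in DT_GIFT_EventList, or non-empty data, then forward to client events.
; The client event looks up the row's LogLine and passes it on as custom data, written through DWLogString to the Modding channel at IMPORTANT level.
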(event Custom|Client_SendCustomData
  (params (Data :type String))
  (Class|LoggerLibrary|DWLogString Data "Modding" "INFOL_IMPORTANT"))

(event Custom|Client_CallToysEvent
  (params (Event :type Name))
  (bind _returnvalue (Utilities|GetDataTableRow "/Game/ModsShared/ConanInterfaceForToys/DataTables/DT_GIFT_EventList.DT_GIFT_EventList" Event)
    (:then
      (CallFunction|ClientSendCustomData (Utilities|Struct|BreakST_GIFT_EventList _returnvalue)))))

(event EventISendCustomData
  (params (Data :type String))
  (if (> (Utilities|String|Len Data) 0)
    (CallFunction|ClientSendCustomData Data)))

(event EventICallToysEvent
  (params (Event :type Name))
  (Utilities|GetDataTableRow "/Game/ModsShared/ConanInterfaceForToys/DataTables/DT_GIFT_EventList.DT_GIFT_EventList" Event
    (:then
      (CallFunction|ClientCallToysEvent Event))))